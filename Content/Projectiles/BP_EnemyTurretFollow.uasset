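; BP_EnemyTurretFollow is a damageable enemy turret that fires a projectile on a looping timer and chases the player character.
; When a BP_BaseCharacter enters its sphere, looping timers lerp it horizontally toward the character with sweep and smoothly yaw it to face them.
; Leaving the sphere clears only the rotation timer, so following continues.
; Detour logic for avoiding other turrets is disconnected leftover code.
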(event OnComponentBeginOverlap(Sphere)
  (params (OverlappedComponent :type Primitive%20Component%20Object%20Reference) (OtherActor :type Actor%20Object%20Reference) (OtherComp :type Primitive%20Component%20Object%20Reference) (OtherBodyIndex :type Integer) (bFromSweep :type Boolean) (SweepResult :type Hit%20Result%20Structure%20%28by%20ref%29))
  (bind _asbp_base_character (Utilities|Casting|CastToBP_BaseCharacter OtherActor))
  (Variables|Default|SetCharacter%20Reference _asbp_base_character)
  (bind _returnvalue (Utilities|Time|SetTimerbyEvent (delegate Custom|Rotate) 0.01 true))
  (Variables|Default|SetTimer%20Handle _returnvalue)
  (if (not (Variables|Default|GetTakingDetour))
    (Utilities|Time|SetTimerbyEvent (delegate Custom|Follow) 0.02 true)))

(event OnComponentEndOverlap(Sphere)
  (params (OverlappedComponent :type Primitive%20Component%20Object%20Reference) (OtherActor :type Actor%20Object%20Reference) (OtherComp :type Primitive%20Component%20Object%20Reference) (OtherBodyIndex :type Integer))
  (Utilities|Casting|CastToBP_BaseCharacter OtherActor)
  (Utilities|Time|ClearandInvalidateTimerbyHandle (Variables|Default|GetTimer%20Handle)))

(event OnComponentBeginOverlap(AntiClip)
  (params (OverlappedComponent :type Primitive%20Component%20Object%20Reference) (OtherActor :type Actor%20Object%20Reference) (OtherComp :type Primitive%20Component%20Object%20Reference) (OtherBodyIndex :type Integer) (bFromSweep :type Boolean) (SweepResult :type Hit%20Result%20Structure%20%28by%20ref%29))
  ;[0.15 0.15 0.15 0.5] Old Dead Code
)

(event Custom|Shoot
  (Game|SpawnActorfromClass "/Game/Projectiles/BP_BaseProjectile.BP_BaseProjectile_C" (Transformation|GetWorldTransform (Variables|Default|GetProjectile%20Arrow)) "Undefined" "MultiplyWithRoot" 0 0))

(event Custom|Rotate
  (Transformation|SetActorRotation (Math|Rotator|MakeRotator 0.0 0.0 (.yaw (Math|Interpolation|RInterpTo (Transformation|GetActorRotation) (Math|Rotator|FindLookatRotation (Transformation|GetActorLocation) (Transformation|GetActorLocation (Variables|Default|GetCharacter%20Reference))) (Utilities|Time|GetWorldDeltaSeconds) 1e+01)))))

(event Custom|Detour
  (bind _returnvalue (Transformation|GetActorTransform))
  (bind _returnvalue_2 (Transformation|GetActorLocation))
  (bind _returnvalue_3 (Transformation|GetActorLocation))
  (bind _returnvalue_4 (Transformation|GetActorLocation))
  (bind _collision_point (Variables|Default|GetCollision%20Point))
  (bind _returnvalue_5 (- _returnvalue_2 _collision_point))
  (bind _returnvalue_6 (+ _returnvalue_3 _returnvalue_5))
  ;[0.15 0.15 0.15 0.5] More Code that (I think) is dead
  (Transformation|SetActorTransform (Math|Transform|MakeTransform (.location (Math|Transform|Lerp(Transform) (Math|Transform|MakeTransform (Math|Vector|MakeVector (.x _returnvalue_4) (.y _returnvalue_4) (.z _returnvalue_4)) "0, 0, 0" "1.000000,1.000000,1.000000") (Math|Transform|MakeTransform (Math|Vector|MakeVector (.x _returnvalue_6) (.y _returnvalue_6) (.z _returnvalue_4)) "0, 0, 0" "1.000000,1.000000,1.000000") 0.005)) (.rotation _returnvalue) (.scale _returnvalue))))

(event Custom|Stop%20Detour
  ;[0.15 0.15 0.15 0.5] Old Dead Code
  (Development|PrintText "Not Taking Detour!")
  (Variables|Default|SetTakingDetour false))

(event Custom|Follow
  (bind _returnvalue (Transformation|GetActorLocation))
  (bind _returnvalue_2 (Transformation|GetActorTransform))
  (bind _character_reference (Variables|Default|GetCharacter%20Reference))
  (bind _returnvalue_3 (Transformation|GetActorLocation _character_reference))
  (Transformation|SetActorTransform (Math|Transform|MakeTransform (.location (Math|Transform|Lerp(Transform) (Math|Transform|MakeTransform (Math|Vector|MakeVector (.x _returnvalue) (.y _returnvalue) (.z _returnvalue)) "0, 0, 0" "1.000000,1.000000,1.000000") (Math|Transform|MakeTransform (Math|Vector|MakeVector (.x _returnvalue_3) (.y _returnvalue_3) (.z _returnvalue)) "0, 0, 0" "1.000000,1.000000,1.000000") 0.005)) (.rotation _returnvalue_2) (.scale _returnvalue_2)) true))

(event Game|Damage|EventAnyDamage
  (params (Damage :type Float%20%28single-precision%29) (DamageType :type Damage%20Type%20Object%20Reference) (InstigatedBy :type Controller%20Object%20Reference) (DamageCauser :type Actor%20Object%20Reference))
  (bind _output_get (Variables|Default|SetHeath (- (Variables|Default|GetHeath) Damage)))
  (if (<= _output_get 0.0)
    (Actor|DestroyActor)))

(event EventBeginPlay
  (Utilities|Time|SetTimerbyEvent (delegate Custom|Shoot) 4.0 true))

(fn ConstructionScript)