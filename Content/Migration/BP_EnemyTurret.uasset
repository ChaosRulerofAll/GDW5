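; BP_EnemyTurret is a destructible enemy turret that fires projectiles and turns to face nearby characters.
; A looping timer from BeginPlay spawns BP_BaseProjectile at ProjectileArrow every few seconds, whether or not a target is present.
; A BP_BaseCharacter entering the Sphere starts a fast timer that interpolates yaw toward it; leaving clears that timer.
; AnyDamage reduces health and destroys the turret at zero.
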(event OnComponentBeginOverlap(Sphere)
  (params (OverlappedComponent :type Primitive%20Component%20Object%20Reference) (OtherActor :type Actor%20Object%20Reference) (OtherComp :type Primitive%20Component%20Object%20Reference) (OtherBodyIndex :type Integer) (bFromSweep :type Boolean) (SweepResult :type Hit%20Result%20Structure%20%28by%20ref%29))
  (bind _asbp_base_character (Utilities|Casting|CastToBP_BaseCharacter OtherActor))
  (Variables|Default|SetCharacter%20Reference _asbp_base_character)
  (bind _returnvalue (Utilities|Time|SetTimerbyEvent (delegate Custom|Rotate) 0.01 true))
  (Variables|Default|SetTimer%20Handle _returnvalue))

(event OnComponentEndOverlap(Sphere)
  (params (OverlappedComponent :type Primitive%20Component%20Object%20Reference) (OtherActor :type Actor%20Object%20Reference) (OtherComp :type Primitive%20Component%20Object%20Reference) (OtherBodyIndex :type Integer))
  (Utilities|Casting|CastToBP_BaseCharacter OtherActor)
  (Utilities|Time|ClearandInvalidateTimerbyHandle (Variables|Default|GetTimer%20Handle)))

(event Custom|Shoot
  (Game|SpawnActorfromClass "/Game/Projectiles/BP_BaseProjectile.BP_BaseProjectile_C" (Transformation|GetWorldTransform (Variables|Default|GetProjectile%20Arrow)) "Undefined" "MultiplyWithRoot" 0 0))

(event Custom|Rotate
  (Transformation|SetActorRotation (Math|Rotator|MakeRotator 0.0 0.0 (.yaw (Math|Interpolation|RInterpTo (Transformation|GetActorRotation) (Math|Rotator|FindLookatRotation (Transformation|GetActorLocation) (Transformation|GetActorLocation (Variables|Default|GetCharacter%20Reference))) (Utilities|Time|GetWorldDeltaSeconds) 1e+01)))))

(event Game|Damage|EventAnyDamage
  (params (Damage :type Float%20%28single-precision%29) (DamageType :type Damage%20Type%20Object%20Reference) (InstigatedBy :type Controller%20Object%20Reference) (DamageCauser :type Actor%20Object%20Reference))
  (bind _output_get (Variables|Default|SetHeath (- (Variables|Default|GetHeath) Damage)))
  (if (<= _output_get 0.0)
    (Actor|DestroyActor)))

(event EventBeginPlay
  (Utilities|Time|SetTimerbyEvent (delegate Custom|Shoot) 4.0 true))

(fn ConstructionScript)